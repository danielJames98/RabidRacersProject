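; CP1 is a race checkpoint that serves as the lap line, counting laps and ending the race after three.
; When a BaseCar0 enters Box at checkpoint zero, it advances the checkpoint, plays a sound, then increments the lap or finishes.
; Finishing disables player input, destroys the checkpoint and notifies VehicleGameMode.
; Box overlaps at any other checkpoint flag the car as going backwards, while Box1 clears that flag.
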(event `self.Box.OnComponentBeginOverlap`
  (params (OverlappedComponent :type "PrimitiveComponent Object Reference") (OtherActor :type "Actor Object Reference") (OtherComp :type "PrimitiveComponent Object Reference") (OtherBodyIndex :type Integer) (bFromSweep :type Boolean) (SweepResult :type "HitResult Structure (by ref)"))
  (bind _asbase_car_0 (cast `/Game/BaseCar0` OtherActor))
  (bind _currentcheckpoint (`/Game/BaseCar0.CurrentCheckpoint` _asbase_car_0))
  (if (== _currentcheckpoint 0)
    ;[1 1 1] Updates checkpoint
    (set `/Game/BaseCar0.CurrentCheckpoint` (+ _currentcheckpoint 1) _asbase_car_0)
    (`GameplayStatics.PlaySound2D` "/Game/UIAssets/bloop.bloop" 0.1 1.0 0.0 null null)
    (bind _returnvalue (+ (`/Game/BaseCar0.CurrentLap` _asbase_car_0) 1))
    (if (== _returnvalue 4)
      ;[1 1 1] Checks if 3 laps completed if true then
      (`self.DisableInput` (`GameplayStatics.GetPlayerController` 0) null)
      (`self.K2_DestroyActor`)
      (bind _asvehicle_game_mode (cast `/Game/GM/VehicleGameMode` (`GameplayStatics.GetGameMode`)))
      (`/Game/GM/VehicleGameMode.FinishedCollided` _asvehicle_game_mode)
      (`self.DisableInput` (`GameplayStatics.GetPlayerPawn` 0) null)
      (`/Game/GM/VehicleGameMode.debugtimechecker` _asvehicle_game_mode)
      (else
        (set `/Game/BaseCar0.CurrentLap` _returnvalue _asbase_car_0)
        (set `/Game/BaseCar0.Backwards?` 0 _asbase_car_0)))
    (else
      ;[1 1 1] checks if players is going wrong way
      (set `/Game/BaseCar0.Backwards?` 1 _asbase_car_0))))

(event `self.Box1.OnComponentBeginOverlap`
  (params (OverlappedComponent :type "PrimitiveComponent Object Reference") (OtherActor :type "Actor Object Reference") (OtherComp :type "PrimitiveComponent Object Reference") (OtherBodyIndex :type Integer) (bFromSweep :type Boolean) (SweepResult :type "HitResult Structure (by ref)"))
  (bind _asbase_car_0 (cast `/Game/BaseCar0` OtherActor))
  (set `/Game/BaseCar0.Backwards?` 0 _asbase_car_0))

(fn `UserConstructionScript`)