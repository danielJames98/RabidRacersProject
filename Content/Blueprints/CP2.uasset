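; CP2 is a checkpoint actor for a car race that tracks a BaseCar0's progress and flags wrong-way driving.
; Overlapping Box advances CurrentCheckpoint and clears Backwards only when the car's count matches the hard-coded preceding checkpoint; otherwise it sets Backwards.
; A second trigger, Box1, always clears the car's Backwards flag on overlap.
; All state lives on the car, so the checkpoint only writes to it.
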(event `self.Box.OnComponentBeginOverlap`
  (params (OverlappedComponent :type "PrimitiveComponent Object Reference") (OtherActor :type "Actor Object Reference") (OtherComp :type "PrimitiveComponent Object Reference") (OtherBodyIndex :type Integer) (bFromSweep :type Boolean) (SweepResult :type "HitResult Structure (by ref)"))
  (bind _asbase_car_0 (cast `/Game/BaseCar0` OtherActor))
  (bind _currentcheckpoint (`/Game/BaseCar0.CurrentCheckpoint` _asbase_car_0))
  (if (== _currentcheckpoint 1)
    (set `/Game/BaseCar0.CurrentCheckpoint` (+ _currentcheckpoint 1) _asbase_car_0)
    (set `/Game/BaseCar0.Backwards?` 0 _asbase_car_0)
    (else
      (set `/Game/BaseCar0.Backwards?` 1 _asbase_car_0))))

(event `self.Box1.OnComponentBeginOverlap`
  (params (OverlappedComponent :type "PrimitiveComponent Object Reference") (OtherActor :type "Actor Object Reference") (OtherComp :type "PrimitiveComponent Object Reference") (OtherBodyIndex :type Integer) (bFromSweep :type Boolean) (SweepResult :type "HitResult Structure (by ref)"))
  (bind _asbase_car_0 (cast `/Game/BaseCar0` OtherActor))
  (set `/Game/BaseCar0.Backwards?` 0 _asbase_car_0))

(fn `UserConstructionScript`)