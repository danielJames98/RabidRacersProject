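; Time crate pickup that temporarily freezes the game timer when its Box is overlapped.
; On overlap it pauses the VehicleGameMode's GameTimer, toggles the five-second UI and hides itself.
; After its TimeToStop duration it resumes the timer, then reappears following a short delay.
; The overlapping actor is not filtered, and hiding does not disable collision.
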(event `self.Box.OnComponentBeginOverlap`
  (params (OverlappedComponent :type "PrimitiveComponent Object Reference") (OtherActor :type "Actor Object Reference") (OtherComp :type "PrimitiveComponent Object Reference") (OtherBodyIndex :type Integer) (bFromSweep :type Boolean) (SweepResult :type "HitResult Structure (by ref)"))
  (bind _game_timer (`/Game/GM/VehicleGameMode.Game timer` (`self.Gamemode`)))
  (bind _asvehicle_game_mode (cast `/Game/GM/VehicleGameMode` (`GameplayStatics.GetGameMode`)))
  (set `self.Gamemode` _asvehicle_game_mode)
  (`KismetSystemLibrary.K2_PauseTimerHandle` _game_timer)
  (`/Game/GM/VehicleGameMode.5secondUiToggle` _asvehicle_game_mode)
  ;[1 1 1] stops timer according to what crate player collided with
  (`self.SetActorHiddenInGame` true)
  (`KismetSystemLibrary.Delay` (`KismetMathLibrary.Conv_IntToDouble` (`self.TimeToStop`)))
  (`KismetSystemLibrary.K2_UnPauseTimerHandle` _game_timer)
  (`KismetSystemLibrary.Delay` 2.0)
  (`self.SetActorHiddenInGame` false))

(fn `UserConstructionScript`)