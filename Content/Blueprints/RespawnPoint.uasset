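; RespawnPoint is a checkpoint actor that records a respawn transform when its trigger box is overlapped.
; A BaseCar0 overlap captures the RespawnSphere's location and yaw-adjusted rotation, then hides the checkpoint temporarily.
; A second Sequence branch writes the stored transform to the "check" SavePoint slot, creating the save if absent.
; That save branch sits outside the car cast, so it runs for any overlapping actor.
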(event `self.TriggerBox.OnComponentBeginOverlap`
  (params (OverlappedComponent :type "PrimitiveComponent Object Reference") (OtherActor :type "Actor Object Reference") (OtherComp :type "PrimitiveComponent Object Reference") (OtherBodyIndex :type Integer) (bFromSweep :type Boolean) (SweepResult :type "HitResult Structure (by ref)"))
  (bind _respawn_sphere (`self.Respawn sphere`))
  (bind (_relativerotation_roll _relativerotation_pitch _relativerotation_yaw) (`KismetMathLibrary.BreakRotator` (`SceneComponent.RelativeRotation` _respawn_sphere)))
  (`|ExecutionSequence`
    (:`then_0`
      (bind _asbase_car_0 (cast `/Game/BaseCar0` OtherActor))
      (set `self.PlayerLoc` (`SceneComponent.K2_GetComponentLocation` _respawn_sphere))
      (set `self.PlayerRot` (`KismetMathLibrary.MakeRotator` _relativerotation_roll _relativerotation_pitch (+ _relativerotation_yaw -90.0)))
      (`self.SetActorHiddenInGame` true)
      (`KismetSystemLibrary.Delay` 10.0)
      (`self.SetActorHiddenInGame` false))
    (:`then_1`
      (bind _returnvalue (`GameplayStatics.DoesSaveGameExist` "check"))
      (if _returnvalue
        (bind _returnvalue_2 (`GameplayStatics.LoadGameFromSlot` "check"))
        (bind _assave_point (cast `/Game/GM/SavePoint` _returnvalue_2))
        (set `/Game/GM/SavePoint.PlayerLocation` (`self.PlayerLoc`) _assave_point)
        (set `/Game/GM/SavePoint.PlayerRotation` (`self.PlayerRot`) _assave_point)
        (`GameplayStatics.SaveGameToSlot` _assave_point "check")
        (else
          (bind _returnvalue_3 (`GameplayStatics.CreateSaveGameObject` "/Game/GM/SavePoint.SavePoint_C"))
          (set `/Game/GM/SavePoint.PlayerLocation` (`self.PlayerLoc`) _returnvalue_3)
          (set `/Game/GM/SavePoint.PlayerRotation` (`self.PlayerRot`) _returnvalue_3)
          (`GameplayStatics.SaveGameToSlot` _returnvalue_3 "check"))))))

(fn `UserConstructionScript`)