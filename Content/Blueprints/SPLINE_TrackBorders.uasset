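; Spline-driven track border actor that tiles a static mesh along a user-drawn spline in the Construction Script, with no active runtime logic.
; The mesh's X bounds set the section length, and only as many whole sections as fit the spline are created.
; Each spline mesh component gets the material instance and spline-sampled endpoints, with tangents clamped to section length for smooth joins.
; An optional flag mirrors sections through negative scale.
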(fn `UserConstructionScript`
  (bind _userspline (`self.UserSpline`))
  (bind _returnvalue (`KismetMathLibrary.Conv_IntToDouble` (`self.SectionSize`)))
  (bind _returnvalue_2 (`StaticMesh.GetBoundingBox` (`self.StaticMesh (Aligned on +X)`)))
  ;[1 1 1] Calculate how many sections will fill the spline.
  (bind _output_get (set `self.SectionSize` (`KismetMathLibrary.FTrunc` (- (.x (`.Max` (break `Box` _returnvalue_2))) (.x (break `Box` _returnvalue_2))))))
  (bind _output_get_2 (set `self.Spline Length` (`SplineComponent.GetSplineLength` (`self.UserSpline`))))
  (bind _returnvalue_3 (`KismetMathLibrary.Conv_IntToDouble` _output_get))
  (bind _output_get_3 (set `self.Number Of sections` (`.ReturnValue` (`KismetMathLibrary.FMod` _output_get_2 _returnvalue_3))))
  (for _index (range _output_get_3)
    (bind _returnvalue_4 (`AddComponent|NODE_AddSplineMeshComponent-0`))
    ;[1 1 1] Set mesh and material parameters
    (`StaticMeshComponent.SetStaticMesh` _returnvalue_4 (`self.StaticMesh (Aligned on +X)`))
    (`PrimitiveComponent.SetMaterial` _returnvalue_4 0 (`self.Material Instance`))
    (`PrimitiveComponent.SetMaterial` _returnvalue_4 0 (`self.Material Instance`))
    (bind _returnvalue_5 (* _index _returnvalue_3))
    (bind _returnvalue_6 (+ _returnvalue_5 _returnvalue_3))
    ;[1 1 1] Fini
    (`SplineMeshComponent.SetStartAndEnd` _returnvalue_4 (`SplineComponent.GetLocationAtDistanceAlongSpline` _userspline _returnvalue_5 "Local") (`KismetMathLibrary.ClampVectorSize` (`SplineComponent.GetTangentAtDistanceAlongSpline` _userspline _returnvalue_5 "Local") 0.0 _returnvalue) (`SplineComponent.GetLocationAtDistanceAlongSpline` _userspline _returnvalue_6 "Local") (`KismetMathLibrary.ClampVectorSize` (`SplineComponent.GetTangentAtDistanceAlongSpline` _userspline _returnvalue_6 "Local") 0.0 _returnvalue) true)
    (if (`self.FlipMesh`)
      (`SplineMeshComponent.SetStartScale` _returnvalue_4 (-1.0 1.0) true)
      (`SplineMeshComponent.SetEndScale` _returnvalue_4 (-1.0 1.0) true))))